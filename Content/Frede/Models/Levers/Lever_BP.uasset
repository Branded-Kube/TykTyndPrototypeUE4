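; Lever actor that the player activates by pressing GrapObject while Frede_RasBallPlayer2 overlaps it.
; Overlap begin and end open and close a gate on the input, which sets Activated and plays a metal bang at world origin.
; Logic deriving Activated from handle pitch and calling IUse on LinkedObject is disconnected, so pressing does not trigger the linked object.
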(event EventTick
  (params (DeltaSeconds :type Float%20%28single-precision%29)))

(event Collision|EventActorBeginOverlap
  (params (OtherActor :type Actor%20Object%20Reference))
  (Utilities|Casting|CastToFrede_RasBallPlayer2 OtherActor)
  (Utilities|FlowControl|Gate true) ; enters at Open
)

(event Collision|EventActorEndOverlap
  (params (OtherActor :type Actor%20Object%20Reference))
  (Utilities|Casting|CastToFrede_RasBallPlayer2 OtherActor)
  (Utilities|FlowControl|Gate true) ; enters at Close
)

(event EventBeginPlay
  (Input|EnableInput (Game|GetPlayerController 0)))

(event Input|ActionEvents|InputActionGrapObject
  (params (Key :type Key%20Structure :default "None"))
  (:Pressed
    (Utilities|FlowControl|Gate true
      (:Exit
        (Variables|Default|SetActivated true)
        (Audio|PlaySoundatLocation "/Game/Frede/Sounds/metal-bang01.metal-bang01" "0, 0, 0" "0, 0, 0" 1.0 1.0 0.0 0 0 0)))))

(fn ConstructionScript)