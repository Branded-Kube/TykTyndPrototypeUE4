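; Player controller for a ball racing game that owns the lap HUD and tracks the current lap.
; BeginPlay creates the LapInfo widget, adds it to the viewport and caches the RasBallPlayer2 pawn.
; UpdateLap advances the lap counter and its text until the race completes, then calls LapTimeCheck and prints the text.
; Race timing, respawn, restart, goal and save/load events and functions are empty stubs, including LapTimeCheck.
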(event Custom|SetChecks)

(event Custom|StartGameSetup)

(event Custom|Restart)

(event Custom|UpdateLap
  ;[1 1 1] Update Lap
  (if (Variables|Default|GetRaceComplete)
    _
    (else
      (bind _output_get (Variables|ValueVariables|SetActualLap (+ (Variables|ValueVariables|GetActualLap) 1)))
      (bind _output_get_2 (Variables|TextVariables|SetCurrentLapText (Utilities|Text|ToText(Integer) _output_get)))))
  (CallFunction|LapTimeCheck)
  (Development|PrintText _output_get_2))

(event Custom|RespawnPlayer)

(event Custom|StartRaceTime)

(event Custom|StopRaceTime)

(event Custom|StartLapTime)

(event Custom|StopLapTime)

(event EventBeginPlay
  (bind _returnvalue (UserInterface|CreateWidget "/Game/MasterLevel/LapInfo.LapInfo_C"))
  (bind _output_get (Variables|Default|SetHudRef _returnvalue))
  (UserInterface|Viewport|AddtoViewport _output_get 0)
  (bind _asras_ball_player_2 (Utilities|Casting|CastToRasBallPlayer2 (Game|Player|GetPlayerPawn 0)))
  (Variables|Default|SetPlayer%20Ref _asras_ball_player_2))

(fn ConstructionScript)

(fn InitText)

(fn SaveGameCheck)

(fn SavetheGame)

(fn LoadtheGame)

(fn LapTimeCheck)

(fn UpdateGoals)